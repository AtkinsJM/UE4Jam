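; BP_Hero is a hero character Blueprint that tracks health and takes damage.
; AnyDamage passes the negated damage to UpdateHealth, which adjusts Health without clamping and checks IsAlive, though the death branch is empty.
; InitialiseHero derives MaxHealth from Level and fills Health, but its only call is unconnected, so it never runs.
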(event EventBeginPlay)

(event Collision|EventActorBeginOverlap
  (params (OtherActor :type Actor%20Object%20Reference)))

(event EventTick
  (params (DeltaSeconds :type Float%20%28single-precision%29)))

(event Game|Damage|EventAnyDamage
  (params (Damage :type Float%20%28single-precision%29) (DamageType :type Damage%20Type%20Object%20Reference) (InstigatedBy :type Controller%20Object%20Reference) (DamageCauser :type Actor%20Object%20Reference))
  (CallFunction|UpdateHealth (* -1 Damage)))

(fn ConstructionScript)

(fn InitialiseHero
  (bind _output_get (Variables|Default|SetMaxHealth (* (Variables|Default|GetLevel) 1e+02)))
  (Variables|Default|SetHealth _output_get))

(fn UpdateHealth
  (params (Value :type Float%20%28single-precision%29))
  (Variables|Default|SetHealth (+ Value (Variables|Default|GetHealth)))
  (if (not (CallFunction|IsAlive))
    _))

(fn IsAlive
  (return (> (Variables|Default|GetHealth) 0.0)))