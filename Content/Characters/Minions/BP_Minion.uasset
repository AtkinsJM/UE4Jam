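; BP_Minion is the minion character Blueprint, handling health, a floating health bar and death.
; Damage feeds UpdateHealth, which refreshes the WBP_FloatingHealthBar_Minion widget and calls Die once health runs out.
; Die requires an AIController, unpossesses it, spawns DeathActor at the minion's transform and destroys the minion.
; Each tick points the bar at the player camera, keeping the widget's own Y in the target to avoid sideways turning.
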(event EventBeginPlay
  (bind _aswbp_floating_health_bar_minion (Utilities|Casting|CastToWBP_FloatingHealthBar_Minion (UserInterface|GetUserWidgetObject (Variables|Default|GetWidget))))
  (bind _output_get (Variables|Default|SetHealth%20Bar _aswbp_floating_health_bar_minion))
  (bind _output_get_2 (Variables|Default|SetHealth (Variables|Default|GetMax%20Health)))
  (bind _output_get_3 (Variables|/Game/UI/WBP_FloatingHealthBar_Minion.WBP_FloatingHealthBar_Minion_C|SetMax%20Health _output_get _output_get_2))
  (bind _output_get_4 (Variables|/Game/UI/WBP_FloatingHealthBar_Minion.WBP_FloatingHealthBar_Minion_C|SetHealth _output_get _output_get_3))
  (Default|UpdateHealthBar _output_get _output_get_4))

(event Collision|EventActorBeginOverlap
  (params (OtherActor :type Actor%20Object%20Reference)))

(event EventTick
  (params (DeltaSeconds :type Float%20%28single-precision%29))
  (CallFunction|RotateHealthBartoCamera))

(event Game|Damage|EventAnyDamage
  (params (Damage :type Float%20%28single-precision%29) (DamageType :type Damage%20Type%20Object%20Reference) (InstigatedBy :type Controller%20Object%20Reference) (DamageCauser :type Actor%20Object%20Reference))
  (CallFunction|UpdateHealth (* -1 Damage)))

(fn ConstructionScript)

(fn UpdateHealth
  (params (Value :type Float%20%28single-precision%29))
  (bind _output_get (Variables|Default|SetHealth (+ Value (Variables|Default|GetHealth))))
  (Default|UpdateHealthBar (Variables|Default|GetHealth%20Bar) _output_get)
  (if (not (CallFunction|IsAlive))
    (CallFunction|Die)))

(fn IsAlive
  (return (> (Variables|Default|GetHealth) 0.0)))

(fn Die
  (bind _asaicontroller (Utilities|Casting|CastToAIController (Pawn|GetController)))
  (Pawn|UnPossess _asaicontroller)
  (Game|SpawnActorfromClass (Variables|Default|GetDeath%20Actor) (Transformation|GetActorTransform) "Undefined" 0 0)
  (Actor|DestroyActor))

(fn RotateHealthBartoCamera
  (bind _returnvalue (Game|GetPlayerCameraManager 0))
  (bind _widget (Variables|Default|GetWidget))
  (bind _returnvalue_2 (Camera|GetCameraLocation _returnvalue))
  (bind _returnvalue_3 (Transformation|GetWorldLocation _widget))
  (Transformation|SetWorldRotation _widget (Math|Rotator|FindLookatRotation (Math|Vector|MakeVector (.x _returnvalue_3) (.y _returnvalue_3) (.z _returnvalue_3)) (Math|Vector|MakeVector (.x _returnvalue_2) (.y _returnvalue_3) (.z _returnvalue_2))) false false))