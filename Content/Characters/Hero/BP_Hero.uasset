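; BP_Hero is an AI-controlled hero character with level-scaled health and a floating health bar.
; BeginPlay computes health from base health and level, then initializes the bar widget, which AnyDamage updates as damage lands.
; Tick turns the bar toward the camera, keeping the target at the widget's own Y.
; At zero health it unpossesses its AI controller, spawns a corpse wearing its skeletal mesh, and destroys itself.
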(event EventBeginPlay
  (CallFunction|InitialiseHero)
  (bind _aswbp_floating_health_bar_hero (Utilities|Casting|CastToWBP_FloatingHealthBar_Hero (UserInterface|GetUserWidgetObject (Variables|Default|GetWidget))))
  (bind _output_get (Variables|Default|SetHealth%20Bar _aswbp_floating_health_bar_hero))
  (bind _output_get_2 (Variables|/Game/UI/WBP_FloatingHealthBar_Hero.WBP_FloatingHealthBar_Hero_C|SetMax%20Health _output_get (Variables|Default|GetHealth)))
  (bind _output_get_3 (Variables|/Game/UI/WBP_FloatingHealthBar_Hero.WBP_FloatingHealthBar_Hero_C|SetHealth _output_get _output_get_2))
  (Default|UpdateHealthBar _output_get _output_get_3))

(event Collision|EventActorBeginOverlap
  (params (OtherActor :type Actor%20Object%20Reference)))

(event EventTick
  (params (DeltaSeconds :type Float%20%28single-precision%29))
  (CallFunction|RotateHealthBartoCamera))

(event Game|Damage|EventAnyDamage
  (params (Damage :type Float%20%28single-precision%29) (DamageType :type Damage%20Type%20Object%20Reference) (InstigatedBy :type Controller%20Object%20Reference) (DamageCauser :type Actor%20Object%20Reference))
  (CallFunction|UpdateHealth (* -1 Damage)))

(fn ConstructionScript)

(fn InitialiseHero
  (bind _output_get (Variables|Default|SetMaxHealth (+ (Variables|Default|GetBase%20Health) (* (Variables|Default|GetLevel) 5e+02))))
  (Variables|Default|SetHealth _output_get))

(fn UpdateHealth
  (params (Value :type Float%20%28single-precision%29))
  (bind _output_get (Variables|Default|SetHealth (+ Value (Variables|Default|GetHealth))))
  (Default|UpdateHealthBar (Variables|Default|GetHealth%20Bar) _output_get)
  (if (not (CallFunction|IsAlive))
    (CallFunction|Die)))

(fn IsAlive
  (return (> (Variables|Default|GetHealth) 0.0)))

(fn RotateHealthBartoCamera
  (bind _returnvalue (Game|GetPlayerCameraManager 0))
  (bind _widget (Variables|Default|GetWidget))
  (bind _returnvalue_2 (Camera|GetCameraLocation _returnvalue))
  (bind _returnvalue_3 (Transformation|GetWorldLocation _widget))
  (Transformation|SetWorldRotation _widget (Math|Rotator|FindLookatRotation (Math|Vector|MakeVector (.x _returnvalue_3) (.y _returnvalue_3) (.z _returnvalue_3)) (Math|Vector|MakeVector (.x _returnvalue_2) (.y _returnvalue_3) (.z _returnvalue_2))) false false))

(fn Die
  (bind _asaicontroller (Utilities|Casting|CastToAIController (Pawn|GetController)))
  (Pawn|UnPossess _asaicontroller)
  (bind _returnvalue (Game|SpawnActorfromClass (Variables|Default|GetDeath%20Actor) (Transformation|GetActorTransform) "Undefined" 0 0))
  (bind _asbp_hero_corpse (Utilities|Casting|CastToBP_HeroCorpse _returnvalue))
  (Class|SkinnedMeshComponent|SetSkeletalMesh (Variables|/Game/Characters/Hero/BP_HeroCorpse.BP_HeroCorpse_C|GetSkeletalMesh _asbp_hero_corpse) (Variables|/Script/Engine.SkinnedMeshComponent|GetSkeletalMesh (Variables|Character|GetMesh)) true)
  (Actor|DestroyActor))