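; Custom game mode that spawns the hero character when play begins.
; It takes the transform of the first BP_HeroStart actor found in the level as the spawn point.
; It then spawns the Hero class there and gives its skeletal mesh a random pick from the HeroMeshes array, so the hero's look varies between sessions.
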(event EventBeginPlay
  (CallFunction|SetHeroSpawnTransform)
  (CallFunction|SpawnHero))

(event EventTick
  (params (DeltaSeconds :type Float%20%28single-precision%29)))

(fn ConstructionScript)

(fn SpawnHero
  (bind _hero_meshes (Variables|Default|GetHero%20Meshes))
  (bind _returnvalue (Game|SpawnActorfromClass (Variables|Default|GetHero) (Variables|Default|GetHero%20Spawn%20Transform) "Undefined" 0 0))
  (Class|SkinnedMeshComponent|SetSkeletalMesh (Variables|/Script/Engine.Character|GetMesh _returnvalue) (Utilities|Array|Get(acopy) _hero_meshes (Math|Random|RandomInteger (Utilities|Array|Length _hero_meshes))) true))

(fn SetHeroSpawnTransform
  (bind _outactors (Actor|GetAllActorsOfClass "/Game/BP_HeroStart.BP_HeroStart_C"))
  (Variables|Default|SetHero%20Spawn%20Transform (Transformation|GetActorTransform (Utilities|Array|Get(acopy) _outactors))))