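; BP_Chest is a destructible chest prop that breaks when its health runs out.
; AnyDamage feeds negated damage into UpdateHealth, which adjusts Health and checks IsAlive.
; When health reaches zero or below, Die spawns the configurable DeathActor at the chest's transform and destroys the chest.
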(event EventBeginPlay)

(event Collision|EventActorBeginOverlap
  (params (OtherActor :type Actor%20Object%20Reference)))

(event EventTick
  (params (DeltaSeconds :type Float%20%28single-precision%29)))

(event Game|Damage|EventAnyDamage
  (params (Damage :type Float%20%28single-precision%29) (DamageType :type Damage%20Type%20Object%20Reference) (InstigatedBy :type Controller%20Object%20Reference) (DamageCauser :type Actor%20Object%20Reference))
  (CallFunction|UpdateHealth (* -1 Damage)))

(fn ConstructionScript)

(fn UpdateHealth
  (params (Value :type Float%20%28single-precision%29))
  (Variables|Default|SetHealth (+ Value (Variables|Default|GetHealth)))
  (if (not (CallFunction|IsAlive))
    (CallFunction|Die)))

(fn IsAlive
  (return (> (Variables|Default|GetHealth) 0.0)))

(fn Destroy
  (Actor|DestroyActor))

(fn Die
  (Game|SpawnActorfromClass (Variables|Default|GetDeath%20Actor) (Transformation|GetActorTransform) "Undefined" 0 0)
  (Actor|DestroyActor))