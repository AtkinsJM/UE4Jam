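; Player controller for an RTS-style camera that passes zoom input through to the camera actor.
; On BeginPlay it finds and caches the first BP_RTSCamera in the level, then forwards the Camera Zoom axis value to that camera's ZoomCamera function.
; An unconnected leftover node chain that moved the camera component along its relative X axis directly never runs.
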(event EventBeginPlay
  (bind _outactors (Actor|GetAllActorsOfClass "/Game/BP_RTSCamera.BP_RTSCamera_C"))
  (Variables|Default|SetCamera_0 (Utilities|Array|Get(acopy) _outactors)))

(event EventTick
  (params (DeltaSeconds :type Float%20%28single-precision%29)))

(event Input|AxisEvents|InputAxisCameraZoom
  (params (AxisValue :type Float%20%28single-precision%29))
  (Class|RTSCamera|ZoomCamera (Variables|Default|GetCamera_0) AxisValue))

(fn ConstructionScript)